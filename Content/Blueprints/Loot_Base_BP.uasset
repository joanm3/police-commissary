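; Loot_Base_BP is a base loot pickup actor with a Vial mesh that can be highlighted and collected.
; The construction script creates a dynamic material instance on the Vial and stores it as MatInst.
; ActivationFeedback toggles the LootActivationParam scalar on that material to switch the activation visual and prints a debug string.
; GetLoot simply destroys the actor, and the event graph holds no active logic.
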(event EventBeginPlay)

(event Collision|EventActorBeginOverlap
  (params (OtherActor :type Actor%20Object%20Reference)))

(event EventTick
  (params (DeltaSeconds :type Float%20%28single-precision%29)))

(fn ConstructionScript
  (bind _vial (Variables|Default|GetVial))
  (bind _returnvalue (Rendering|Material|CreateDynamicMaterialInstance _vial 0 (Rendering|Material|GetMaterial _vial 0) :!class /Script/Engine.PrimitiveComponent))
  (Variables|Default|SetMatInst _returnvalue))

(fn GetLoot
  (Actor|DestroyActor))

(fn ActivationFeedback
  (params (bActivate :type Boolean))
  (bind _matinst (Variables|Default|GetMatInst))
  (Development|PrintString "activation feedback")
  (if bActivate
    (Rendering|Material|SetScalarParameterValue _matinst "LootActivationParam" 1.0 :!class /Script/Engine.MaterialInstanceDynamic)
    (else
      (Rendering|Material|SetScalarParameterValue _matinst "LootActivationParam" 0.0 :!class /Script/Engine.MaterialInstanceDynamic))))