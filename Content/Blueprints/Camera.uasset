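; Security camera that sweeps its lens side to side on a looping or timed yaw timeline and detects the player.
; Each tick it checks cone overlaps, then line-traces to confirm the player pawn is the first hit.
; Detection pauses the sweep, recolors the light and yaws the lens toward the player within clamped limits.
; A retriggerable delay restores the scan color and resumes the sweep once the player stays undetected.
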(event Custom|EventPlayerDetected
  (Utilities|FlowControl|Sequence
    (:then_0
      (CallFunction|StartDetection)
      (bind (_direction _camerarotation) (Timeline|TimelineCameraYawn Stop)
        (:Update
          (Transformation|SetRelativeRotation (Variables|Default|GetCamera_Lens) (Math|Rotator|MakeRotator 0.0 (Variables|Camera|GetPitchRot) (* _camerarotation (Variables|Camera|GetMaxYawnRot))) false false))))
    (:then_1
      (Utilities|FlowControl|RetriggerableDelay 2.0)
      (CallFunction|ResetDetection)
      (Timeline|TimelineCameraYawn Play))))

(event EventBeginPlay
  (Components|Timeline|SetPlayRate (Variables|Default|GetTimelineCameraYawn) (Variables|Camera|GetRotPlayRate))
  (bind (_direction _camerarotation) (Timeline|TimelineCameraYawn Play)
    (:Update
      (Transformation|SetRelativeRotation (Variables|Default|GetCamera_Lens) (Math|Rotator|MakeRotator 0.0 (Variables|Camera|GetPitchRot) (* _camerarotation (Variables|Camera|GetMaxYawnRot))) false false))))

(event EventTick
  (params (DeltaSeconds :type Float%20%28single-precision%29))
  (CallFunction|PlayerDetection)
  (if (Variables|Default|GetPlayerDetected)
    (CallFunction|FollowPlayer)))

(fn ConstructionScript
  (Transformation|SetRelativeRotation (Variables|Default|GetCamera_Lens) (Math|Rotator|MakeRotator 0.0 (Variables|Camera|GetPitchRot) 0.0) false false)
  (Rendering|Components|Light|SetLightColor (Variables|Default|Getlight) (Variables|Camera|GetScanColor) true))

(fn PlayerDetection
  (bind _cone (Variables|Default|Getcone))
  (bind _overlappingactors (Collision|GetOverlappingActors _cone "/Game/Blueprints/PlayerPawn.PlayerPawn_C" :!class /Script/Engine.PrimitiveComponent))
  (if (> (Utilities|Array|Length _overlappingactors) 0)
    (bind _outhit (Collision|LineTraceForObjects (Transformation|GetWorldLocation (Variables|Default|Getcone)) (Transformation|GetActorLocation (Utilities|Array|Get(acopy) _overlappingactors)) (Utilities|Array|MakeArray "ObjectTypeQuery1" "ObjectTypeQuery3") false 0 "ForOneFrame"))
    (Utilities|Casting|CastToPlayerPawn (.HitActor (Collision|BreakHitResult _outhit)))
    (CallFunction|EventPlayerDetected)))

(fn StartDetection
  (Variables|Default|SetPlayerDetected true)
  (Rendering|Components|Light|SetLightColor (Variables|Default|Getlight) (Variables|Default|GetDetectedColor) true))

(fn ResetDetection
  (Variables|Default|SetPlayerDetected false)
  (Rendering|Components|Light|SetLightColor (Variables|Default|Getlight) (Variables|Camera|GetScanColor) true))

(fn FollowPlayer
  (bind _maxyawnrot (Variables|Camera|GetMaxYawnRot))
  (Transformation|SetRelativeRotation (Variables|Default|GetCamera_Lens) (Math|Rotator|MakeRotator 0.0 (Variables|Camera|GetPitchRot) (Math|Float|Clamp(Float) (.Yaw (Math|Rotator|BreakRotator (Math|Rotator|MakeRotfromX (Math|Vector|Normalize (- (Transformation|GetActorLocation (Game|Player|GetPlayerPawn 0)) (Transformation|GetWorldLocation (Variables|Default|GetCamera_Lens))))))) (* _maxyawnrot -1.0) _maxyawnrot)) false false))