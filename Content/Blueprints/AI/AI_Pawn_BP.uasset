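; Stealth AI pawn that patrols linked points and escalates through Patrol, Suspicious, Search and Alert states as it detects actors.
; While activated, Tick polls AIPerception and fills a detection meter weighted by distance, facing and noise-maker speed, switching states at AIStateTunning thresholds.
; Move-completed events drive waypoint waits, investigation of detected actors and Search routes built from nearby reachable search points.
; Player contact triggers Alert directly, and BeginPlay attaches a state UI widget.
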(event OnComponentHit(CapsuleComponent)
  (params (HitComponent :type Primitive%20Component%20Object%20Reference) (OtherActor :type Actor%20Object%20Reference) (OtherComp :type Primitive%20Component%20Object%20Reference) (NormalImpulse :type Vector :default "0, 0, 0") (Hit :type Hit%20Result%20Structure%20%28by%20ref%29))
  ;[1 1 1] IA Behavior
  ;;[1 1 1] Touched by player
  (Utilities|Casting|CastToCharacter_Pawn OtherActor
    (:then
      _)
    (:CastFailed
      (Utilities|Casting|CastToPlayerPawn OtherActor)))
  (CallFunction|TouchbyPlayer))

(event Custom|Event_Move_Completed
  (params (RequestID :type AI%20Request%20ID%20Structure) (Result :type EPathFollowingResult%20Enum))
  (bind _currentwaittime (Variables|Default|GetCurrentWaitTime))
  ;[1 1 1] IA Behavior
  ;;[1 1 1] ReachTargetBehavior
  (switch Utilities|FlowControl|Switch|SwitchonEPathFollowingResult Result
    (:Success
      _)
    (:Blocked
      _))
  (switch Utilities|FlowControl|Switch|SwitchonE_AI_State (Variables|Default|GetAIState)
    (:NewEnumerator0
      _)
    (:NewEnumerator1
      _)
    (:NewEnumerator2
      _))
  (if (Variables|Default|GetbCheckPosition)
    (Variables|Default|SetbCheckPosition false)
    (Utilities|FlowControl|RetriggerableDelay _currentwaittime)
    (CallFunction|CreateSearchPatrol)
    (else
      (Default|PointReached (Variables|Default|GetCurrentTarget) self)
      (if (> (Variables|Default|GetCurrentWaitTime) 0.0)
        (Transformation|SetWorldRotation (Variables|Collision|GetCapsuleComponent) (Variables|Default|GetWaitRotation) false false))
      (Utilities|FlowControl|RetriggerableDelay _currentwaittime)))
  (if (not (Variables|Default|GetbCheckPosition))
    (switch Utilities|FlowControl|Switch|SwitchonE_AI_State (Variables|Default|GetAIState)
      (:NewEnumerator0
        _)
      (:NewEnumerator1
        _)
      (:NewEnumerator2
        _))
    (CallFunction|FindNextPatrolTarget)
    (CallFunction|MovetoNextPatrolPoint)))

(event Custom|Debug_Undetected
  ;[1 1 1] IA Behavior
  (Variables|AI|SetActivate (not (Variables|AI|GetActivate))))

(event Custom|BeginPatrol
  (params (Patrol%20Point :type AI%20Point%20Patrol%20BP%20Object%20Reference))
  ;[1 1 1] IA Behavior
  ;;[1 1 1] Level Event
  (bind _output_get (Variables|AI|SetPatrolStart Patrol%20Point))
  (bind _output_get_2 (Variables|Default|SetCurrentTarget _output_get))
  (CallFunction|MoveActor _output_get_2))

(event Custom|PausePatrol
  ;[1 1 1] IA Behavior
  ;;[1 1 1] Level Event
  (AI|Navigation|StopMovement (Variables|Default|GetAIController)))

(event Custom|ResumePatrol
  ;[1 1 1] IA Behavior
  ;;[1 1 1] Level Event
  (bind _asai_point_patrol_bp (Utilities|Casting|CastToAI_Point_Patrol_BP (Variables|Default|GetCurrentTarget)))
  (CallFunction|MoveActor _asai_point_patrol_bp))

(event EventBeginPlay
  ;[1 1 1] IA Behavior
  ;;[1 1 1] Initialization
  (CallFunction|ChangeAIState "NewEnumerator0")
  (CallFunction|InitAI)
  (EventDispatchers|BindEventtoReceiveMoveCompleted (Variables|Default|GetAIController) (delegate Custom|Event_Move_Completed)))

(event EventTick
  (params (DeltaSeconds :type Float%20%28single-precision%29))
  ;[1 1 1] IA Behavior
  ;;[1 1 1] UpdateDetection
  (if (Variables|AI|GetActivate)
    (switch Utilities|FlowControl|Switch|SwitchonE_AI_State (Variables|Default|GetAIState)
      (:NewEnumerator0
        (CallFunction|UpdateDetectedActor :!label _label)
        (CallFunction|UpdateDetection DeltaSeconds)
        (CallFunction|UpdateStateChange))
      (:NewEnumerator1
        (goto _label))
      (:NewEnumerator2
        (goto _label))
      (:NewEnumerator3
        (Default|CallEDStartAlert)))))

(fn ConstructionScript)

(fn MovetoNextPatrolPoint
  (bind _patrolstart (Variables|AI|GetPatrolStart))
  (Utilities|IsValid (Variables|Default|GetCurrentTarget)
    (:Is%20Valid
      _)
    (:Is%20Not%20Valid
      (Utilities|IsValid _patrolstart
        (:Is%20Valid
          (Variables|Default|SetCurrentTarget _patrolstart)))))
  (AI|Navigation|MovetoActor (Variables|Default|GetAIController) (Variables|Default|GetCurrentTarget) 4e+01 true true false)
  (Variables|Default|SetCurrentWaitTime (Variables|/Game/Blueprints/AI/AI_Point_BP.AI_Point_BP_C|GetWaitTime (Variables|Default|GetCurrentTarget)))
  (Variables|Default|SetWaitRotation (Transformation|GetActorRotation (Variables|Default|GetCurrentTarget))))

(fn ChangeAIState
  (params (NewState :type E_AI_State%20Enum))
  (bind _output_get (Variables|Default|SetAIState NewState))
  (Variables|/Script/Engine.CharacterMovementComponent|SetMaxWalkSpeed (Variables|Character|GetCharacterMovement) (select (Variables|Default|GetbIsCrouched) (/ (Utilities|Select :Index _output_get :NewEnumerator0 1e+02 :NewEnumerator1 1e+02 :NewEnumerator2 2e+02 :NewEnumerator3 0.0) 2.0) (Utilities|Select :Index _output_get :NewEnumerator0 1e+02 :NewEnumerator1 1e+02 :NewEnumerator2 2e+02 :NewEnumerator3 0.0)))
  (switch Utilities|FlowControl|Switch|SwitchonE_AI_State _output_get
    (:NewEnumerator0
      _)
    (:NewEnumerator3
      (Variables|Default|SetbCheckPosition false)))
  (Components|Activation|Activate (Variables|Default|GetAIPerception) false))

(fn UpdateDetection
  (params (DTime :type Float%20%28single-precision%29))
  (bind _currentaistatebar (Variables|Default|GetCurrentAIStateBar))
  (bind (_state _previousstate _nextstate _limitup _limitdown _speedincreasestatefactor _speeddecreasestatefactor) (Utilities|Struct|BreakS_AI_StateTransition _currentaistatebar))
  (Utilities|IsValid (Variables|Default|GetActorSeen)
    (:Is%20Valid
      (Utilities|FlowControl|Sequence
        (:then_0
          (if (Variables|Default|GetbSightStimuli)
            (Variables|Default|SetStateProgression (+ (Variables|Default|GetStateProgression) (* (CallFunction|SpeedVisualDetectionFactor) DTime _speedincreasestatefactor)))
            (CallFunction|StartCheck "0, 0, 0" :!label _label)))
        (:then_1
          (if (Variables|Default|GetbHearingStimuli)
            (Variables|Default|SetStateProgression (CallFunction|ClampMaxProgression (+ (Variables|Default|GetStateProgression) (* (CallFunction|SpeedHearingDetectionFactor) DTime 5e+01))))
            (goto _label)))))
    (:Is%20Not%20Valid
      (if (and (not (Variables|Default|GetbCheckPosition)) (== (Utilities|Array|Length (Variables|Default|GetPatrolSearch)) 0))
        (if (> (- (Variables|Default|GetStateProgression) (* DTime _speeddecreasestatefactor)) 0.0)
          (Variables|Default|SetStateProgression (- (Variables|Default|GetStateProgression) (* DTime _speeddecreasestatefactor)))
          (else
            (Variables|Default|SetStateProgression 0.0)))))))

(fn UpdateAIState
  (params (NewState :type E_AI_State%20Enum))
  (bind (_patrol _suspicious _search _alert) (Utilities|GetClassDefaults "/Game/Blueprints/AI/AIStateTunning.AIStateTunning_C"))
  (switch Utilities|FlowControl|Switch|SwitchonE_AI_State NewState
    (:NewEnumerator0
      (Variables|Default|SetCurrentAIStateBar _patrol))
    (:NewEnumerator1
      (Variables|Default|SetCurrentAIStateBar _suspicious))
    (:NewEnumerator2
      (Variables|Default|SetCurrentAIStateBar _search)
      (CallFunction|StartCheck "0, 0, 0" :!label _label))
    (:NewEnumerator3
      (Variables|Default|SetCurrentAIStateBar _alert)
      (goto _label))))

(fn InitAI
  (bind _patrolstart (Variables|AI|GetPatrolStart))
  (Variables|Default|SetCurrentAIStateBar (.Patrol (Utilities|GetClassDefaults "/Game/Blueprints/AI/AIStateTunning.AIStateTunning_C")))
  (bind _returnvalue (UserInterface|CreateWidget "/Game/Blueprints/AI/UI_AIState.UI_AIState_C"))
  (UserInterface|Viewport|AddtoViewport _returnvalue 0)
  (Variables|/Game/Blueprints/AI/UI_AIState.UI_AIState_C|SetAIAttached _returnvalue self)
  (bind _asaicontroller (Utilities|Casting|CastToAIController (Pawn|GetController)))
  (Variables|Default|SetAIController _asaicontroller)
  (Utilities|IsValid _patrolstart
    (:Is%20Valid
      (bind _output_get (Variables|Default|SetCurrentTarget _patrolstart))
      (CallFunction|MoveActor _output_get))))

(fn SpeedVisualDetectionFactor
  (bind _returnvalue (Math|Float|MakeLiteralFloat 1.5e+03))
  (bind _self self)
  (bind _actorseen (Variables|Default|GetActorSeen))
  (Utilities|IsValid _actorseen
    (:Is%20Valid
      (return (* (Math|Float|Power (- (Math|Float|MakeLiteralFloat 1.0) (/ (Math|Float|Clamp(Float) (Transformation|GetDistanceTo _actorseen self) 0.0 _returnvalue) _returnvalue)) 2.0) (Math|Float|Square (+ (Math|Float|MakeLiteralFloat 1.0) (Math|Float|Clamp(Float) (Math|Vector|DotProduct (Math|Vector|Normalize (- (Transformation|GetActorLocation (Variables|Default|GetActorSeen)) (Transformation|GetActorLocation _self))) (Math|Vector|Normalize (Math|Vector|GetForwardVector (Variables|Collision|GetCapsuleComponent _self))))))))))
    (:Is%20Not%20Valid
      (return 0.0))))

(fn CreateSearchPatrol
  (bind _searchpointpatrolsize (Variables|Default|GetSearchPointPatrolSize))
  (bind _searchpatrol (LocalVariables|GetSearchPatrol))
  (if (Utilities|Enum|Equal(Enum) (Variables|Default|GetAIState) "NewEnumerator2")
    (Utilities|Array|Clear (Variables|Default|GetPatrolSearch))
    (bind _outactors (Actor|GetAllActorsOfClass "/Game/Blueprints/AI/AI_Point_Search_BP.AI_Point_Search_BP_C"))
    (for _array_element _outactors
      (if (and (Utilities|Enum|Equal(Enum) (.ReturnValue (Class|NavigationSystem|GetPathCost (Transformation|GetActorLocation self) (Transformation|GetActorLocation _array_element))) "Success") (< (Transformation|GetDistanceTo _array_element self) (Variables|Default|GetMaxSearchDistance)))
        (Utilities|Array|Add (LocalVariables|GetSearchPatrol) _array_element)))
    (if (> (Utilities|Array|Length _searchpatrol) _searchpointpatrolsize)
      (Utilities|Array|Resize _searchpatrol _searchpointpatrolsize))
    (bind _output_get (Variables|Default|SetPatrolSearch _searchpatrol))
    (Variables|Default|SetCurrentTarget (Utilities|Array|Get(acopy) _output_get))))

(fn UpdateStateChange
  (bind _currentaistatebar (Variables|Default|GetCurrentAIStateBar))
  (bind _currentaistatebar_2 (Variables|Default|GetCurrentAIStateBar))
  (bind (_state _previousstate _nextstate) (Utilities|Struct|BreakS_AI_StateTransition _currentaistatebar_2))
  (bind (_state_2 _previousstate_2 _nextstate_2 _limitup _limitdown) (Utilities|Struct|BreakS_AI_StateTransition _currentaistatebar))
  (Utilities|FlowControl|Sequence
    (:then_0
      (if (> (Variables|Default|GetStateProgression) (Math|Conversions|ToFloat(Integer) _limitup))
        (CallFunction|UpdateAIState _nextstate)
        (CallFunction|ChangeAIState _state :!label _label)))
    (:then_1
      (if (< (Variables|Default|GetStateProgression) (Math|Conversions|ToFloat(Integer) _limitdown))
        (CallFunction|UpdateAIState _previousstate)
        (goto _label)))))

(fn StartCheck
  (params (CheckPosition :type Vector))
  (bind _actorseen (Variables|Default|GetActorSeen))
  (switch Utilities|FlowControl|Switch|SwitchonE_AI_State (Variables|Default|GetAIState)
    (:NewEnumerator1
      _)
    (:NewEnumerator2
      _))
  (if (Math|Vector|Equal(Vector) CheckPosition "0, 0, 0" 0.0001)
    (Utilities|IsValid _actorseen
      (:Is%20Valid
        (Variables|Default|SetbCheckPosition true)
        (Variables|Default|SetCurrentWaitTime (Variables|Default|GetCheckPositionDelay))
        (AI|Navigation|MovetoLocation (Variables|Default|GetAIController) (Transformation|GetActorLocation _actorseen) 1.5e+02 true true false)))
    (else
      (Variables|Default|SetbCheckPosition true)
      (Variables|Default|SetCurrentWaitTime (Variables|Default|GetCheckPositionDelay))
      (AI|Navigation|MovetoLocation (Variables|Default|GetAIController) CheckPosition 1.5e+02 true true false))))

(fn UpdateDetectedActor
  (bind _aiperception (Variables|Default|GetAIPerception))
  (bind _outactors (Class|AIPerceptionComponent|GetPerceivedActors _aiperception "/Script/AIModule.AISense_Hearing"))
  (Utilities|FlowControl|Sequence
    (:then_0
      (bind _filteredarray (Utilities|Array|FilterArray (Class|AIPerceptionComponent|GetPerceivedActors _aiperception "/Script/AIModule.AISense_Sight") "/Game/Blueprints/AI/StimuliActor_BP.StimuliActor_BP_C"))
      (Utilities|ArrayEmpty _filteredarray
        (:Not%20Empty
          (Variables|Default|SetbSightStimuli true))
        (:Empty
          (Variables|Default|SetbSightStimuli false)))
      (LocalVariables|SetPerceivedActor _filteredarray))
    (:then_1
      (bind _filteredarray_2 (Utilities|Array|FilterArray _outactors "/Game/Interaction/Blueprints/Pawn/Player/Character_Pawn.Character_Pawn_C"))
      (Utilities|ArrayEmpty _filteredarray_2
        (:Not%20Empty
          (Variables|Default|SetbHearingStimuli true)
          (Utilities|Array|AppendArray (LocalVariables|GetPerceivedActor) _outactors))
        (:Empty
          (Variables|Default|SetbHearingStimuli false))))
    (:then_2
      (Utilities|IsValid (Utilities|Array|Get(acopy) (LocalVariables|GetPerceivedActor))
        (:Is%20Valid
          (bind _output_get (Variables|Default|SetActorSeen (Utilities|Array|Get(acopy) (LocalVariables|GetPerceivedActor))))
          (Class|AIPerceptionComponent|GetActorsPerception (Variables|Default|GetAIPerception) _output_get))
        (:Is%20Not%20Valid
          (if (Variables|Default|GetbCheckPosition)
            (switch Utilities|FlowControl|Switch|SwitchonE_AI_State (Variables|Default|GetAIState)
              (:NewEnumerator1
                _)))
          (Variables|Default|SetActorSeen 0))))))

(fn SpeedHearingDetectionFactor
  (bind _returnvalue (Math|Float|MakeLiteralFloat 1.5e+03))
  (bind _self self)
  (bind _actorseen (Variables|Default|GetActorSeen))
  (bind _actorseen_2 (Variables|Default|GetActorSeen))
  (bind _returnvalue_2 (Transformation|GetDistanceTo _actorseen_2 _self))
  (if (< _returnvalue_2 _returnvalue)
    (bind _ascharacter_pawn (Utilities|Casting|CastToCharacter_Pawn _actorseen)
      (:then
        (return (* (Math|Float|Power (- (Math|Float|MakeLiteralFloat 1.0) (/ _returnvalue_2 _returnvalue)) 2.0) (Math|Float|Power (/ (Math|Float|Clamp(Float) (Math|Vector|VectorLength (Transformation|GetVelocity _ascharacter_pawn)) 0.0 (Variables|/Script/Engine.CharacterMovementComponent|GetMaxWalkSpeed (Variables|/Script/Engine.Character|GetCharacterMovement _ascharacter_pawn))) (Variables|/Script/Engine.CharacterMovementComponent|GetMaxWalkSpeed (Variables|/Script/Engine.Character|GetCharacterMovement _ascharacter_pawn))) 2.0) 1e+01)))
      (:CastFailed
        (Utilities|Casting|CastToPlayerPawn _actorseen
          (:then
            (return (* (Math|Float|Power (- (Math|Float|MakeLiteralFloat 1.0) (/ _returnvalue_2 _returnvalue)) 2.0) (Math|Float|Power (/ (Math|Float|Clamp(Float) (Math|Vector|VectorLength (Transformation|GetVelocity _ascharacter_pawn)) 0.0 (Variables|/Script/Engine.CharacterMovementComponent|GetMaxWalkSpeed (Variables|/Script/Engine.Character|GetCharacterMovement _ascharacter_pawn))) (Variables|/Script/Engine.CharacterMovementComponent|GetMaxWalkSpeed (Variables|/Script/Engine.Character|GetCharacterMovement _ascharacter_pawn))) 2.0) 1e+01)))
          (:CastFailed
            _)))))
  (return 0.0))

(fn FindNextPatrolTarget
  (bind _asai_point_patrol_bp (Utilities|Casting|CastToAI_Point_Patrol_BP (Variables|Default|GetCurrentTarget))
    (:then
      (Utilities|IsValid (Variables|/Game/Blueprints/AI/AI_Point_Patrol_BP.AI_Point_Patrol_BP_C|GetNextPatrolPoint _asai_point_patrol_bp)
        (:Is%20Valid
          (Variables|Default|SetCurrentTarget (Variables|/Game/Blueprints/AI/AI_Point_Patrol_BP.AI_Point_Patrol_BP_C|GetNextPatrolPoint _asai_point_patrol_bp)))
        (:Is%20Not%20Valid
          (Variables|Default|SetCurrentTarget 0))))
    (:CastFailed
      (Utilities|Casting|CastToAI_Point_Search_BP (Variables|Default|GetCurrentTarget)
        (:then
          (if (> (Utilities|Array|Length (Variables|Default|GetPatrolSearch)) 0)
            (Variables|Default|SetCurrentTarget (Utilities|Array|Get(acopy) (Variables|Default|GetPatrolSearch)))
            (Utilities|Array|RemoveIndex (Variables|Default|GetPatrolSearch))
            (else
              (Variables|Default|SetCurrentTarget 0 :!label _label))))
        (:CastFailed
          (goto _label))))))

(fn ClampMaxProgression
  (params (Value :type Float%20%28single-precision%29))
  (return (Math|Float|Clamp(Float) Value 0.0 (Math|Conversions|ToFloat(Integer) (.LimitUp (Utilities|Struct|BreakS_AI_StateTransition (.Search (Utilities|GetClassDefaults "/Game/Blueprints/AI/AIStateTunning.AIStateTunning_C"))))))))

(fn TouchbyPlayer
  (switch Utilities|FlowControl|Switch|SwitchonE_AI_State (Variables|Default|GetAIState)
    (:NewEnumerator0
      _)
    (:NewEnumerator1
      _)
    (:NewEnumerator2
      _))
  (CallFunction|ChangeAIState "NewEnumerator3")
  (Components|Activation|Deactivate (Variables|Default|GetAIPerception)))

(fn MoveActor
  (params (PatrolPoint :type AI%20Point%20BP%20Object%20Reference))
  (AI|Navigation|MovetoActor (Variables|Default|GetAIController) PatrolPoint 5e+01 true true))